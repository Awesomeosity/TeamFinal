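; Actor that links the Santa game to Twitch, letting chat viewers trigger reindeer-named effects on the player.
; On BeginPlay it shows an in-game browser login, then connects TwitchPlay to the user's channel and registers chat commands, re-prompting on failure.
; Commands call player character, game mode or music manager functions, then show a reindeer notification and particle burst.
; It also forwards chat to SantaGameState and reposts help on a looping timer.
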(event Custom|UserAuthenticatedEvent
  (params (bAuthenticated :type Boolean))
  (bind _twitchauth (Variables|Default|GetTwitchAuth))
  (bind _twitchplay (Variables|Default|GetTwitchPlay))
  (bind _returnvalue (Class|TwitchAuthComponent|GetUser _twitchauth))
  (bind _name (Utilities|Struct|BreakTwitchUser _returnvalue))
  ;[1 1 1 1 24] Set up the Twitch integration
  (if bAuthenticated
    ;;[0.3827 0.4142 1] Retrieve and authenticate user info
    (Development|PrintString _name)
    (Class|TwitchIRCComponent|SetUserInfo (Variables|Default|GetTwitchPlay) (Utilities|String|Append "oauth:" (Class|TwitchAuthComponent|GetAccessToken _twitchauth)) _name _name)
    (bind (__out_error _returnvalue_2) (Class|TwitchIRCComponent|Connect _twitchplay))
    (if _returnvalue_2
      (bind (__out_error_2 _returnvalue_3) (Class|TwitchIRCComponent|AuthenticateTwitchIRC _twitchplay))
      (if _returnvalue_3
        ;;[0.7479 0.1281 1] Set up Twitch commands
        (Class|TwitchPlayComponent|SetupEncapsulationChars _twitchplay "'" "\"")
        (bind __out_result (Class|TwitchPlayComponent|RegisterCommand _twitchplay "help" (delegate Custom|HelpCommand)))
        (Development|PrintString __out_result)
        (bind __out_result_2 (Class|TwitchPlayComponent|RegisterCommand _twitchplay "blitzen" (delegate Custom|BlitzenCommand)))
        (Development|PrintString __out_result_2)
        (bind __out_result_3 (Class|TwitchPlayComponent|RegisterCommand _twitchplay "comet" (delegate Custom|CometCommand)))
        (Development|PrintString __out_result_3)
        (bind __out_result_4 (Class|TwitchPlayComponent|RegisterCommand _twitchplay "dancer" (delegate Custom|DancerCommand)))
        (Development|PrintString __out_result_4)
        (bind __out_result_5 (Class|TwitchPlayComponent|RegisterCommand _twitchplay "prancer" (delegate Custom|PrancerCommand)))
        (Development|PrintString __out_result_5)
        (bind __out_result_6 (Class|TwitchPlayComponent|RegisterCommand _twitchplay "vixen" (delegate Custom|VixenCommand)))
        (Development|PrintString __out_result_6)
        (bind __out_result_7 (Class|TwitchPlayComponent|RegisterCommand _twitchplay "dasher" (delegate Custom|DasherCommand)))
        (Development|PrintString __out_result_7)
        (bind __out_result_8 (Class|TwitchPlayComponent|RegisterCommand _twitchplay "cupid" (delegate Custom|CupidCommand)))
        (Development|PrintString __out_result_8)
        (bind __out_result_9 (Class|TwitchPlayComponent|RegisterCommand _twitchplay "rudolph" (delegate Custom|RudolphCommand)))
        (Development|PrintString __out_result_9)
        (bind __out_result_10 (Class|TwitchPlayComponent|RegisterCommand _twitchplay "donner" (delegate Custom|DonnerCommand)))
        (Development|PrintString __out_result_10)
        ;;[0.898 1 0] Print all Twitch messages to debug
        (EventDispatchers|AssignOnMessageReceived (Variables|Default|GetTwitchPlay) (delegate Custom|TestMessageReceived))
        (Development|PrintString "Twitch setup complete.")
        (Widget|RemovefromParent (Variables|Default|GetSignInWidget))
        (CallFunction|HelpCommand "help" (Utilities|Array|MakeArray "") "AutoBot")
        (Utilities|Time|SetTimerbyFunctionName 0 "LoopHelpMessage" 6e+01 true)
        (bind _assanta_game_state (Utilities|Casting|CastToSantaGameState (Game|GetGameState)))
        (Default|SetTwitchChatAvailable _assanta_game_state)
        (else
          ;;;[1 0 0.03465] An error has occurred connecting to Twitch. Request the user sign in again.
          (Development|PrintString "Authentication failed!")
          (Development|PrintString __out_error_2)
          (CallFunction|RequestLogin :!label _label)))
      (else
        (Development|PrintString "Unable to connect!")
        (Development|PrintString __out_error)
        (goto _label)))
    (else
      ;;[1 0 0.02135] Login failed; try again
      (Development|PrintString "Authentication failed!")
      (CallFunction|RequestLogin))))

(event Custom|HelpCommand
  (params (_command_name :type String) (_command_options :type Array%20of%20Strings) (_sender_username :type String))
  ;[0.004608 1 0 1 24] Respond to the 'help' command
  (Development|PrintString (Utilities|String|Append _sender_username " used the help command."))
  (Class|TwitchIRCComponent|SendIRCMessage (Variables|Default|GetTwitchPlay) "[AUTO MESSAGE] Enter commands as follows: '[insert command here]' (apostrophes included) ________________________________________ There is a command for each reindeer (Dasher, Dancer, Prancer, Vixen, Comet, Cupid, Donner, Blitzen, and Rudolph). ________________________________________ For example, type in 'rudolph' to use the Rudolph command. ________________________________________ Use the 'help' command to see this message again." true (.name (Utilities|Struct|BreakTwitchUser (Class|TwitchAuthComponent|GetUser (Variables|Default|GetTwitchAuth))))))

(event Custom|RudolphCommand
  (params (_command_name :type String) (_command_options :type Array%20of%20Strings) (_sender_username :type String))
  ;[0.2448 0.1706 0.04947] Twitch reindeer commands
  (bind _asthird_person_character (Utilities|Casting|CastToThirdPersonCharacter (Game|Player|GetPlayerPawn 0)))
  (Default|TwitchRudolph _asthird_person_character 10)
  (CallFunction|TwitchReindeerNotification _command_name))

(event Custom|VixenCommand
  (params (_command_name :type String) (_command_options :type Array%20of%20Strings) (_sender_username :type String))
  ;[0.2448 0.1706 0.04947] Twitch reindeer commands
  (bind _asthird_person_character (Utilities|Casting|CastToThirdPersonCharacter (Game|Player|GetPlayerPawn 0)))
  (Default|TwitchVixen _asthird_person_character 10)
  (CallFunction|TwitchReindeerNotification _command_name))

(event Custom|DasherCommand
  (params (_command_name :type String) (_command_options :type Array%20of%20Strings) (_sender_username :type String))
  ;[0.2448 0.1706 0.04947] Twitch reindeer commands
  (bind _asthird_person_character (Utilities|Casting|CastToThirdPersonCharacter (Game|Player|GetPlayerPawn 0)))
  (Default|TwitchDasher _asthird_person_character 10 2.5)
  (CallFunction|TwitchReindeerNotification _command_name))

(event Custom|TestMessageReceived
  (params (_message :type String) (_username :type String))
  (bind _returnvalue (Utilities|String|Append _username ": " _message))
  ;[1 1 1 1 24] Set up the Twitch integration
  ;;[0.898 1 0] Print all Twitch messages to debug
  (if (Utilities|Enum|Equal(Enum) "" _username)
    ;;[0.6727 0.1058 1] Twitch itself sent a message. May or may not inform the user of an error.
    (Development|PrintString _message)
    (bind _assanta_game_state (Utilities|Casting|CastToSantaGameState (Game|GetGameState)))
    (Default|UpdateTwitchChat _assanta_game_state _message)
    (else
      (Development|PrintString _returnvalue)
      (bind _assanta_game_state_2 (Utilities|Casting|CastToSantaGameState (Game|GetGameState)))
      (Default|UpdateTwitchChat _assanta_game_state_2 _returnvalue))))

(event Custom|RequestLogin
  (bind _twitchauth (Variables|Default|GetTwitchAuth))
  ;[0.8057 0.2968 1 1 24] Prompt the player to log in to Twitch through an in-game browser
  (Class|TwitchAuthComponent|ClearAccessToken (Variables|Default|GetTwitchAuth))
  (Widget|RemovefromParent (Variables|Default|GetSignInWidget))
  (UserInterface|Viewport|AddtoViewport (stale EventBeginPlay _output_get) 0)
  (bind _returnvalue (UserInterface|CreateWidget "/Game/Twitch/UI/ReindeerNotification.ReindeerNotification_C" (Game|GetPlayerController 0)))
  (bind _output_get (Variables|Default|SetReindeerNotificationWidget _returnvalue))
  (UserInterface|Viewport|AddtoViewport _output_get 0)
  (Class|TwitchAuthComponent|Authenticate _twitchauth (Variables|/Game/Twitch/UI/BrowserBlueprint.BrowserBlueprint_C|GetTwitchWebBrowser (stale EventBeginPlay _output_get)))
  (EventDispatchers|BindEventtoOnUserAuthenticated _twitchauth (delegate Custom|UserAuthenticatedEvent)))

(event Custom|BlitzenCommand
  (params (_command_name :type String) (_command_options :type Array%20of%20Strings) (_sender_username :type String))
  ;[0.2448 0.1706 0.04947] Twitch reindeer commands
  (bind _astwitch_game_mode (Utilities|Casting|CastToTwitchGameMode (Game|GetGameMode)))
  (Default|CallSignalRunning _astwitch_game_mode)
  (CallFunction|TwitchReindeerNotification _command_name))

(event Custom|CometCommand
  (params (_command_name :type String) (_command_options :type Array%20of%20Strings) (_sender_username :type String))
  ;[0.2448 0.1706 0.04947] Twitch reindeer commands
  (bind _asthird_person_character (Utilities|Casting|CastToThirdPersonCharacter (Game|Player|GetPlayerPawn 0)))
  (Default|TwitchComet _asthird_person_character 1e+03)
  (CallFunction|TwitchReindeerNotification _command_name))

(event Custom|CupidCommand
  (params (_command_name :type String) (_command_options :type Array%20of%20Strings) (_sender_username :type String))
  ;[0.2448 0.1706 0.04947] Twitch reindeer commands
  (bind _asthird_person_character (Utilities|Casting|CastToThirdPersonCharacter (Game|Player|GetPlayerPawn 0)))
  (Default|TwitchCupid _asthird_person_character 10 8e+02)
  (CallFunction|TwitchReindeerNotification _command_name))

(event Custom|DonnerCommand
  (params (_command_name :type String) (_command_options :type Array%20of%20Strings) (_sender_username :type String))
  ;[0.2448 0.1706 0.04947] Twitch reindeer commands
  (bind _outactors (Actor|GetAllActorsOfClass "/Game/music/MusicManager.MusicManager_C"))
  (Default|PlayRandomSong (Utilities|Array|Get(acopy) _outactors))
  (CallFunction|TwitchReindeerNotification _command_name))

(event Custom|DancerCommand
  (params (_command_name :type String) (_command_options :type Array%20of%20Strings) (_sender_username :type String))
  ;[0.2448 0.1706 0.04947] Twitch reindeer commands
  (bind _asthird_person_character (Utilities|Casting|CastToThirdPersonCharacter (Game|Player|GetPlayerPawn 0)))
  (Default|TwitchDancer _asthird_person_character 3)
  (CallFunction|TwitchReindeerNotification _command_name))

(event Custom|PrancerCommand
  (params (_command_name :type String) (_command_options :type Array%20of%20Strings) (_sender_username :type String))
  ;[0.2448 0.1706 0.04947] Twitch reindeer commands
  (bind _asthird_person_character (Utilities|Casting|CastToThirdPersonCharacter (Game|Player|GetPlayerPawn 0)))
  (Default|TwitchPrancer _asthird_person_character 10 3.0)
  (CallFunction|TwitchReindeerNotification _command_name))

(event EventBeginPlay
  (bind _returnvalue (Game|GetPlayerController 0))
  (bind _twitchauth (Variables|Default|GetTwitchAuth))
  ;[0.8057 0.2968 1 1 24] Prompt the player to log in to Twitch through an in-game browser
  (bind _returnvalue_2 (UserInterface|CreateWidget "/Game/Twitch/UI/BrowserBlueprint.BrowserBlueprint_C" _returnvalue))
  (bind _output_get (Variables|Default|SetSignInWidget _returnvalue_2))
  (UserInterface|Viewport|AddtoViewport _output_get 0)
  (bind _returnvalue_3 (UserInterface|CreateWidget "/Game/Twitch/UI/ReindeerNotification.ReindeerNotification_C" _returnvalue))
  (bind _output_get_2 (Variables|Default|SetReindeerNotificationWidget _returnvalue_3))
  (UserInterface|Viewport|AddtoViewport _output_get_2 0)
  (Class|TwitchAuthComponent|Authenticate _twitchauth (Variables|/Game/Twitch/UI/BrowserBlueprint.BrowserBlueprint_C|GetTwitchWebBrowser _output_get))
  (EventDispatchers|BindEventtoOnUserAuthenticated _twitchauth (delegate Custom|UserAuthenticatedEvent)))

(fn ConstructionScript)

(fn LoopHelpMessage
  (CallFunction|HelpCommand "help" (Utilities|Array|MakeArray "") "AutoBot"))

(fn TwitchReindeerNotification
  (params (Reindeer%20Name :type String))
  ;[1 1 1] Send a reindeer across the screen after a command comes in
  (Default|ShowReindeer (Variables|Default|GetReindeerNotificationWidget) (Utilities|String|Append (Class|KismetStringLibrary|ToUpper Reindeer%20Name) "!"))
  (bind _asthird_person_character (Utilities|Casting|CastToThirdPersonCharacter (Game|Player|GetPlayerPawn 0)))
  (bind _returnvalue (Effects|SpawnEmitterAttached 0 (Variables|/Script/Engine.Character|GetMesh _asthird_person_character) "None" "0, 0, 0" "0, 0, 0" "0.100000,0.100000,0.100000"))
  (bind _returnvalue_2 (Utilities|Time|SetTimerbyEvent (EventDispatchers|CreateEvent _returnvalue :!event Deactivate) 3.0))
  (LocalVariables|SetTimer _returnvalue_2))